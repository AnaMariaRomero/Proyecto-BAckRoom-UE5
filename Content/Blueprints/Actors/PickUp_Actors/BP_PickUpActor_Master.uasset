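; Master pickup actor that lets the first-person player add an item and amount to their inventory component.
; A sphere overlap activates per-tick line traces to the player's camera, showing a camera-facing prompt widget when unobstructed.
; The prompt toggles with pickup distance, and input is enabled only within range.
; SecundaryAction calls AddItem, keeping any remainder in the actor; otherwise the actor is destroyed, even if adding fails.
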(event `self.ReceiveTick`
  (params (DeltaSeconds :type "Float (single-precision)"))
  (bind _returnvalue (`GameplayStatics.GetPlayerController` 0))
  (bind _promptwidget (`self.PromptWidget`))
  (bind (_returnvalue_x _returnvalue_y _returnvalue_z) (`KismetMathLibrary.BreakVector` (`SceneComponent.K2_GetComponentLocation` (`self.StaticMesh`))))
  (`SceneComponent.K2_SetWorldLocation` (`self.PromptWidget`) (`KismetMathLibrary.MakeVector` _returnvalue_x _returnvalue_y (+ _returnvalue_z (`self.WidgetDistanceAboveMesh`))) false false)
  (if (`self.UpdateActor`)
    (bind (_outhit _returnvalue_2) (`KismetSystemLibrary.LineTraceSingle` (`self.K2_GetActorLocation`) (`SceneComponent.K2_GetComponentLocation` (`/Game/Blueprints/BP_Game/BP_FirstPersonCharacter.Camera` (`self.Player Ref`))) "TraceTypeQuery1"))
    (if (not _returnvalue_2)
      (`SceneComponent.SetVisibility` _promptwidget true false)
      (`SceneComponent.K2_SetWorldRotation` (`self.PromptWidget`) (`KismetMathLibrary.FindLookAtRotation` (`SceneComponent.K2_GetComponentLocation` (`self.PromptWidget`)) (`SceneComponent.K2_GetComponentLocation` (`/Game/Blueprints/BP_Game/BP_FirstPersonCharacter.Camera` (`self.Player Ref`)))) false false)
      (bind (_bblockinghit _binitialoverlap _time _distance _location _impactpoint _normal _impactnormal _physmat _hitactor _hitcomponent _hitbonename _bonename _hititem _elementindex _faceindex _tracestart _traceend) (`GameplayStatics.BreakHitResult` _outhit))
      (bind _returnvalue_3 (<= (`KismetMathLibrary.VSize` (- _tracestart _traceend)) (`self.PickUpDistance`)))
      (`/Game/UMG/Inventory/W_PickUpPrompt.TogglePrompt` (cast `/Game/UMG/Inventory/W_PickUpPrompt` (`WidgetComponent.GetUserWidgetObject` (`self.PromptWidget`)) :!pure true) _returnvalue_3)
      (if _returnvalue_3
        (`self.EnableInput` _returnvalue)
        (else
          (`self.DisableInput` _returnvalue)))
      (else
        (`SceneComponent.SetVisibility` _promptwidget false false)
        (`self.DisableInput` (`GameplayStatics.GetPlayerController` 0))))))

(event `self.Sphere.OnComponentBeginOverlap`
  (params (OverlappedComponent :type "PrimitiveComponent Object Reference") (OtherActor :type "Actor Object Reference") (OtherComp :type "PrimitiveComponent Object Reference") (OtherBodyIndex :type Integer) (bFromSweep :type Boolean) (SweepResult :type "HitResult Structure (by ref)"))
  (bind _asbp_first_person_character (cast `/Game/Blueprints/BP_Game/BP_FirstPersonCharacter` OtherActor))
  (set `self.Player Ref` _asbp_first_person_character)
  (`SceneComponent.SetVisibility` (`self.PromptWidget`) true false)
  (set `self.UpdateActor` true))

(event `self.Sphere.OnComponentEndOverlap`
  (params (OverlappedComponent :type "PrimitiveComponent Object Reference") (OtherActor :type "Actor Object Reference") (OtherComp :type "PrimitiveComponent Object Reference") (OtherBodyIndex :type Integer))
  (cast `/Game/Blueprints/BP_Game/BP_FirstPersonCharacter` OtherActor)
  (`SceneComponent.SetVisibility` (`self.PromptWidget`) false false)
  (set `self.UpdateActor` false)
  (`self.DisableInput` (`GameplayStatics.GetPlayerController` 0)))

(event `InputAction|SecundaryAction`
  (params (Key :type "Key Structure"))
  (:`Pressed`
    (`KismetSystemLibrary.LogString` "Hello")
    (bind (_success_ _remainder) (`/Game/Blueprints/BlueprintsComponents/BPC_Inventory.AddItem` (`/Game/Blueprints/BP_Game/BP_FirstPersonCharacter.BPC_Inventory` (`self.Player Ref`)) (`self.Item`) (`self.Amount`)))
    (if _success_
      (if (> _remainder 0)
        (set `self.Amount` _remainder)
        (else
          (`self.K2_DestroyActor`)))
      (else
        (`self.K2_DestroyActor`)))))

(fn `UserConstructionScript`
  (`SceneComponent.K2_SetRelativeLocation` (`self.PromptWidget`) (`KismetMathLibrary.MakeVector` 0.0 0.0 (`self.WidgetDistanceAboveMesh`)) false false))