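; Door actor that swings open away from the player when interacted with and closes on the next interaction.
; Interact toggles DoorClosed and, on opening, takes the dot product of the player-to-door direction and the actor's forward vector.
; Its sign picks the swing direction, and a timeline lerps the mesh's relative yaw up to a quarter turn.
; Closing plays the same timeline in reverse.
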(event `/Game/Blueprints/Interfaces/BPI_Interaction.Interact`
  (if (`self.DoorClosed?`)
    (set `self.DoorClosed?` false)
    (set `self.DotProduct` (`KismetMathLibrary.Dot_VectorVector` (`KismetMathLibrary.Normal` (- (`self.K2_GetActorLocation` self) (`self.K2_GetActorLocation` (`self.Player Ref`)))) (`self.GetActorForwardVector` self)))
    (bind (_direction _alpha) (`Timeline|Timeline_0` :!via `PlayFromStart` :!label _label)
      (:`Update`
        (`SceneComponent.K2_SetRelativeRotation` (`self.DoorMesh`) (`KismetMathLibrary.MakeRotator` 0.0 0.0 (`KismetMathLibrary.Lerp` 0.0 (select `bool` (>= (`self.DotProduct`) 0.0) :`false` -90.0 :`true` 90.0) _alpha)) false false)))
    (else
      (set `self.DoorClosed?` true)
      (goto _label :!via `ReverseFromEnd`))))

(fn `UserConstructionScript`
  (`parent.UserConstructionScript`))