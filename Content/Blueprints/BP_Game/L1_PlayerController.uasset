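; L1_PlayerController is a player controller that handles mouse look and toggles the inventory menu.
; On BeginPlay it creates a collapsed inventory widget; toggling it disables movement and look, centers a visible cursor, removes any examination widget, and switches to Game and UI input, reversing on close.
; Look axes apply pitch and yaw scaled by a sensitivity variable, and the Return action fires CallPressedReturn, likely an event dispatcher.
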(event `self.ReceiveBeginPlay`
  (bind _returnvalue (`|CreateWidget` "/Game/UMG/Inventory/W_InventoryMenu.W_InventoryMenu_C"))
  (bind _output_get (set `self.W_InventoryMenu Ref` _returnvalue))
  (`Widget.SetVisibility` _output_get "Collapsed")
  (`UserWidget.AddToViewport` (`self.W_InventoryMenu Ref`) 0))

(event `InputAction|Inventory Toggle`
  (params (Key :type "Key Structure"))
  (:`Pressed`
    (`self.ToggleInventory`)))

(event `ToggleInventory`
  (bind (_returnvalue_x _returnvalue_y) (`KismetMathLibrary.BreakVector2D` (`WidgetLayoutLibrary.GetViewportSize`)))
  (bind _w_inventorymenu_ref (`self.W_InventoryMenu Ref`))
  (bind _w_examinationref (`self.W_ExaminationRef`))
  (bind _charactermovement (`Character.CharacterMovement` (`GameplayStatics.GetPlayerCharacter` 0)))
  (if (`self.IsInventoryOpen?`)
    (set `self.IsInventoryOpen?` false)
    (`CharacterMovementComponent.SetMovementMode` _charactermovement "MOVE_Walking" 0)
    (`self.ResetIgnoreLookInput`)
    (set `self.bShowMouseCursor` false)
    (`Widget.SetVisibility` _w_inventorymenu_ref "Collapsed")
    (`WidgetBlueprintLibrary.SetInputMode_GameOnly` self)
    (else
      (set `self.IsInventoryOpen?` true)
      (`CharacterMovementComponent.DisableMovement` _charactermovement)
      (`self.SetIgnoreLookInput` true)
      (set `self.bShowMouseCursor` true)
      (`self.SetMouseLocation` (`KismetMathLibrary.FTrunc` (/ _returnvalue_x 2.0)) (`KismetMathLibrary.FTrunc` (/ _returnvalue_y 2.0)))
      (`Widget.SetVisibility` _w_inventorymenu_ref "SelfHitTestInvisible")
      (if (`Widget.IsInViewport` _w_examinationref)
        (`Widget.RemoveFromParent` _w_examinationref))
      (`WidgetBlueprintLibrary.SetInputMode_GameAndUIEx` self (`self.W_InventoryMenu Ref`)))))

(event `InputAxis|LookUp`
  (params (AxisValue :type "Float (single-precision)"))
  (`self.AddPitchInput` (* AxisValue (`self.LookSensibility`))))

(event `InputAxis|LookRight`
  (params (AxisValue :type "Float (single-precision)"))
  (`self.AddYawInput` (* AxisValue (`self.LookSensibility`))))

(event `InputAction|Return`
  (params (Key :type "Key Structure"))
  (:`Pressed`
    (`self.PressedReturn`)))

(fn `UserConstructionScript`)