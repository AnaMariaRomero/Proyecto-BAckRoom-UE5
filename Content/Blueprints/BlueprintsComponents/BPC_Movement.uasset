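; Movement component for the player character that handles sprinting with stamina and crouching by changing max walk speed.
; Looping timers drain stamina during sprint while the player moves, then regenerate it after a retriggerable delay once sprinting stops.
; Crouching cancels the sprint timer and has BP_FirstPersonCharacter shorten its capsule; starting a sprint ends the crouch.
; StopSprint is ignored while crouched, so it does not start regeneration then.
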(event `StartSprint`
  (if (`self.IsCrouching?`)
    (`self.EndCrouch`))
  (if (and (> (`self.CurrentStamina`) (`self.MinStamina`)) (> (`KismetMathLibrary.VSize` (`Actor.GetVelocity` (`self.Player Ref`))) 10.0))
    (`KismetSystemLibrary.K2_ClearTimer` null "RegenerateStamina")
    (`self.SetMaxWalkSpeed` (`self.SprintSpeed`))
    (`KismetSystemLibrary.K2_SetTimer` null "SprintTimer" 0.1 true)
    (else
      (`self.StopSprint`))))

(event `SprintTimer`
  (if (and (> (`self.CurrentStamina`) (`self.MinStamina`)) (> (`KismetMathLibrary.VSize` (`Actor.GetVelocity` (`self.Player Ref`))) 10.0))
    (set `self.CurrentStamina` (`KismetMathLibrary.FClamp` (- (`self.CurrentStamina`) 1.0) (`self.MinStamina`) (`self.MaxStamina`)))
    (if (<= (`self.CurrentStamina`) (`self.MinStamina`))
      (`self.StopSprint`))
    (else
      (`self.StopSprint`))))

(event `StopSprint`
  (if (not (`self.IsCrouching?`))
    (`KismetSystemLibrary.K2_ClearTimer` null "SprintTimer")
    (`self.SetMaxWalkSpeed` (`self.WalkSpeed`))
    (`KismetSystemLibrary.RetriggerableDelay` 3.0)
    (if (not (`KismetSystemLibrary.K2_IsTimerActive` null "SprintTimer"))
      (`KismetSystemLibrary.K2_SetTimer` null "RegenerateStamina" 0.03 true))))

(event `RegenerateStamina`
  (set `self.CurrentStamina` (`KismetMathLibrary.FClamp` (+ (`self.CurrentStamina`) 1.0) (`self.MinStamina`) (`self.MaxStamina`)))
  (if (>= (`self.CurrentStamina`) (`self.MaxStamina`))
    (`KismetSystemLibrary.K2_ClearTimer` null "RegenerateStamina")))

(event `StartCrouch`
  (`KismetSystemLibrary.K2_ClearTimer` null "SprintTimer")
  (`self.SetMaxWalkSpeed` (`self.CrouchSpeed`))
  (`/Game/Blueprints/BP_Game/BP_FirstPersonCharacter.ShortenPlayerCapsule` (cast `/Game/Blueprints/BP_Game/BP_FirstPersonCharacter` (`self.Player Ref`) :!pure true))
  (set `self.IsCrouching?` true))

(event `EndCrouch`
  (`self.SetMaxWalkSpeed` (`self.WalkSpeed`))
  (`/Game/Blueprints/BP_Game/BP_FirstPersonCharacter.LenghtenPlayerCapsule` (cast `/Game/Blueprints/BP_Game/BP_FirstPersonCharacter` (`self.Player Ref`) :!pure true))
  (set `self.IsCrouching?` false))

(fn `Initialize`
  (params (Character :type "Character Object Reference"))
  (set `self.Player Ref` Character)
  (set `CharacterMovementComponent.MaxWalkSpeed` (`self.WalkSpeed`) (`Character.CharacterMovement` (`self.Player Ref`))))

(fn `SetMaxWalkSpeed`
  (params (`Max Walk Speed` :type "Float (single-precision)"))
  (set `CharacterMovementComponent.MaxWalkSpeed` `Max Walk Speed` (`Character.CharacterMovement` (`self.Player Ref`))))